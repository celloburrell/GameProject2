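; AI controller for enemy ships in Destroyer5000 that moves its pawn in a zigzag and fires bullets.
; A looping one-second timer flips the lateral direction, while Tick feeds movement input combining that sideways motion with a constant drift along negative world X.
; Tick also runs into a Delay that throttles firing, spawning BP_Bullet at the possessed BP_EnemyShip's BulletSpawn transform roughly every 1.5 seconds.
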(event Custom|SwitchDirection
  ;[1 1 1] Set direction timer
  (Variables|Default|SetMovingRight (not (Variables|Default|GetMovingRight))))

(event EventBeginPlay
  ;[1 1 1] Set direction timer
  (Utilities|Time|SetTimerbyEvent (delegate Custom|SwitchDirection) 1.0 true))

(event EventTick
  (params (DeltaSeconds :type Float%20%28single-precision%29))
  (bind _returnvalue (Pawn|GetControlledPawn))
  ;[1 1 1] Enemy movement and fire
  (Utilities|IsValid _returnvalue
    (:Is%20Valid
      (Class|PawnMovementComponent|AddInputVector (Pawn|GetMovementComponent _returnvalue) (Math|Vector|MakeVector -0.5 (select (Variables|Default|GetMovingRight) 1.0 -1.0) 0.0) false)
      (bind _asbp_enemy_ship (Utilities|Casting|CastToBP_EnemyShip (Pawn|GetControlledPawn)))
      (Utilities|FlowControl|Delay 1.5)
      (Game|SpawnActorfromClass "/Game/BP_Bullet.BP_Bullet_C" (Transformation|GetWorldTransform (Variables|/Game/BP_EnemyShip.BP_EnemyShip_C|GetBulletSpawn _asbp_enemy_ship)) "Undefined" 0 0))))

(fn ConstructionScript)