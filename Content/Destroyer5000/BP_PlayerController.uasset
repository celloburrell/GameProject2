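; BP_PlayerController is the player controller that handles input and the lives display for the player's ship in Destroyer5000.
; On BeginPlay it creates the WBP_Lives widget and adds it to the viewport.
; Each tick it feeds the forward and right axis values as world X and Y input into the controlled pawn's movement component.
; The Fire action casts the pawn to BP_PlayerShip and delegates firing to it.
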(event EventBeginPlay
  ;[1 1 1] Create lives remaining widget
  (bind _returnvalue (UserInterface|CreateWidget "/Game/WBP_Lives.WBP_Lives_C" self))
  (UserInterface|Viewport|AddtoViewport _returnvalue 0))

(event EventTick
  (params (DeltaSeconds :type Float%20%28single-precision%29))
  (bind _returnvalue (Pawn|GetControlledPawn))
  ;[1 1 1] Update controlled pawn's movement with input
  (Utilities|IsValid _returnvalue
    (:Is%20Valid
      (Class|PawnMovementComponent|AddInputVector (Pawn|GetMovementComponent _returnvalue) (Math|Vector|MakeVector (Input|AxisValues|GetForwardMapping) (Input|AxisValues|GetRightMapping) 0.0) false))))

(event Input|ActionEvents|InputActionFire
  (params (Key :type Key%20Structure))
  ;[1 1 1] Fire: Delegate fire to pawn
  (:Pressed
    (bind _asbp_player_ship (Utilities|Casting|CastToBP_PlayerShip (Pawn|GetControlledPawn)))
    (Default|Fire _asbp_player_ship)))

(fn ConstructionScript)