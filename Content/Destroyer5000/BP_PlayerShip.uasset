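; BP_PlayerShip is the player ship in Destroyer5000, and its graph handles shooting.
; The Fire event spawns a BP_Bullet at the Arrow component's world transform and plays the Pew sound.
; A ReadyToFire flag gates each shot, and a one-shot timer calls EnableFire to restore it after CooldownSeconds.
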(event Custom|Fire
  ;[1 1 1] Fire Event for Bullet
  (if (Variables|Default|GetReadyToFire)
    (Game|SpawnActorfromClass "/Game/BP_Bullet.BP_Bullet_C" (Transformation|GetWorldTransform (Variables|Default|GetArrow)) "Undefined" 0 0)
    (Audio|PlaySound2D "/Game/SoundAssets/pew.pew" 1.0 1.0 0.0 0 0)
    (Variables|Default|SetReadyToFire false)
    (Utilities|Time|SetTimerbyEvent (delegate Custom|EnableFire) (Variables|Default|GetCooldownSeconds))))

(event Custom|EnableFire
  ;[1 1 1] Fire Event for Bullet
  (Variables|Default|SetReadyToFire true))

(fn ConstructionScript)