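; BP_Bullet is the projectile in Destroyer5000, resolving hits on enemy and player ships through its Box overlap event.
; An enemy ship hit destroys both ship and bullet and plays a 2D blop sound.
; A player ship hit destroys the bullet and decrements LivesRemaining on the first actor found of that ship's class, reopening the Destroyer5000 level when lives reach zero.
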(event OnComponentBeginOverlap(Box)
  (params (OverlappedComponent :type Primitive%20Component%20Object%20Reference) (OtherActor :type Actor%20Object%20Reference) (OtherComp :type Primitive%20Component%20Object%20Reference) (OtherBodyIndex :type Integer) (bFromSweep :type Boolean) (SweepResult :type Hit%20Result%20Structure%20%28by%20ref%29))
  (bind _returnvalue (Utilities|GetClass OtherActor))
  ;[1 1 1] Bullets destroy enemy ships and then itself
  (if (Utilities|ClassIsChildOf (Utilities|GetClass OtherActor) "/Game/BP_EnemyShip.BP_EnemyShip_C")
    (Actor|DestroyActor OtherActor)
    (Audio|PlaySound2D "/Game/SoundAssets/blop.blop" 1.0 1.0 0.0 0 0)
    (Actor|DestroyActor)
    (else
      ;[1 1 1] Bullets decrement player lives and restart level if player dies
      (if (Utilities|ClassIsChildOf _returnvalue "/Game/BP_PlayerShip.BP_PlayerShip_C")
        (Actor|DestroyActor)
        (bind _outactors (Actor|GetAllActorsOfClass _returnvalue))
        (bind _asbp_player_ship (Utilities|Casting|CastToBP_PlayerShip (Utilities|Array|Get(acopy) _outactors)))
        (bind _output_get (Variables|/Game/BP_PlayerShip.BP_PlayerShip_C|SetLivesRemaining _asbp_player_ship (- (Variables|/Game/BP_PlayerShip.BP_PlayerShip_C|GetLivesRemaining _asbp_player_ship) 1)))
        (if (== _output_get 0)
          (Game|OpenLevel(byName) "/Game/Destroyer5000"))))))

(fn ConstructionScript)